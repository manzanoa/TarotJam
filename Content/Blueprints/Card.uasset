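; Card is a clickable card actor that toggles between two faces when its Cube is clicked.
; It starts unflipped with the checker tile material, and each click inverts IsFlipped and swaps the Cube to the matching floor or checker material.
; An unconnected loop over ConnectedCards, which would set each linked card's material from that card's flip state, never runs.
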(event OnClicked(Cube)
  (params (TouchedComponent :type Primitive%20Component%20Object%20Reference) (ButtonPressed :type Key%20Structure :default "None"))
  (bind _cube (Variables|Default|GetCube))
  (bind _output_get (Variables|Default|SetIsFlipped (not (Variables|Default|GetIsFlipped))))
  (if _output_get
    (Rendering|Material|SetMaterial _cube 0 "/Game/StarterContent/Materials/M_Basic_Floor.M_Basic_Floor")
    (else
      (Rendering|Material|SetMaterial _cube 0 "/Game/StarterContent/Materials/M_Ceramic_Tile_Checker.M_Ceramic_Tile_Checker"))))

(event EventBeginPlay
  (Variables|Default|SetIsFlipped false)
  (Rendering|Material|SetMaterial (Variables|Default|GetCube) 0 "/Game/StarterContent/Materials/M_Ceramic_Tile_Checker.M_Ceramic_Tile_Checker"))

(fn ConstructionScript)